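; Butterfly variant of the pest character in RogueDefense that pollinates a plant instead of damaging it.
; ChooseTarget shuffles all BP_Plant_Base actors, sets the first at one specific growth stage as CurrentTarget, then calls the parent logic.
; Attack replaces the parent behavior, calling Pollinate on the plant and then GoAway.
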(event EventBeginPlay
  (|CallParentFunction) ; This node is disabled and will not be called.\nDrag off pins to build functionality.
)

(event Collision|EventActorBeginOverlap
  (params (OtherActor :type Actor%20Object%20Reference)))

(event EventTick
  (params (DeltaSeconds :type Float%20%28single-precision%29))
  (|CallParentFunction DeltaSeconds) ; This node is disabled and will not be called.\nDrag off pins to build functionality.
)

(fn ConstructionScript
  (|CallParentFunction))

(fn Attack
  (params (Plant :type BP%20Plant%20Base%20Object%20Reference))
  (Default|Pollinate Plant)
  (CallFunction|GoAway false))

(fn ChooseTarget
  (bind _outactors (Actor|GetAllActorsOfClass "/Game/RogueDefense/Blueprints/Plant/Base/BP_Plant_Base.BP_Plant_Base_C"))
  (Utilities|Array|Shuffle _outactors)
  (bind _array_element (Utilities|Array|ForEachLoopwithBreak _outactors :!label _label)
    (:LoopBody
      (if (Utilities|Enum|Equal(Enum) (Variables|/Game/RogueDefense/Blueprints/Plant/Base/BP_Plant_Base.BP_Plant_Base_C|GetGrowthStage _array_element) "NewEnumerator3")
        (Variables|Default|SetCurrentTarget _array_element)
        (goto _label Break)))
    (:Completed
      (|CallParentFunction))))