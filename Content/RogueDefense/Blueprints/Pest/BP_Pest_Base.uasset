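; Base pest actor for RogueDefense that picks a plant to target when it spawns.
; On BeginPlay it sets its widget image to Bug0, then selects the plant with the highest cached grid column from all BP_Plant_Base actors.
; It binds to that plant's death event, but the handler takes no action and Attack is an empty stub.
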(event Custom|CheckIfIAttacked
  (params (Performer :type Actor%20Object%20Reference))
  (if (not (Variables|Default|GetDidIAttack))
    (if (== Performer (Variables|Default|GetTargetPlant))
      _)))

(event EventBeginPlay
  (bind _aswbp_pest (Utilities|Casting|CastToWBP_Pest (UserInterface|GetWidget (Variables|Default|GetWidget))))
  (Default|ChangeImage _aswbp_pest "/Game/RogueDefense/Downloads/Visuals/bug/Bug0.Bug0")
  (CallFunction|ChoosePlant)
  (EventDispatchers|BindEventtoOnDeath (Variables|Default|GetTargetPlant) (delegate Custom|CheckIfIAttacked)))

(event EventTick
  (params (DeltaSeconds :type Float%20%28single-precision%29)))

(fn ConstructionScript)

(fn ChoosePlant
  (LocalVariables|SetPlantTarget%28Local%29 0)
  (bind _outactors (Actor|GetAllActorsOfClass "/Game/RogueDefense/Blueprints/Plant/Base/BP_Plant_Base.BP_Plant_Base_C"))
  (for _array_element _outactors
    (LocalVariables|GetPlantTarget%28Local%29
      (:then
        (if (< (Variables|/Game/RogueDefense/Blueprints/GridLockPosition/BP_GridLockPosition.BP_GridLockPosition_C|GetCol (Variables|/Game/RogueDefense/Blueprints/BP_TouchTest.BP_TouchTest_C|GetCachedGrid (LocalVariables|GetPlantTarget%28Local%29))) (Variables|/Game/RogueDefense/Blueprints/GridLockPosition/BP_GridLockPosition.BP_GridLockPosition_C|GetCol (Variables|/Game/RogueDefense/Blueprints/BP_TouchTest.BP_TouchTest_C|GetCachedGrid _array_element)))
          (LocalVariables|SetPlantTarget%28Local%29 _array_element)))
      (:else
        (LocalVariables|SetPlantTarget%28Local%29 _array_element))))
  (Variables|Default|SetTargetPlant (LocalVariables|GetPlantTarget%28Local%29)))

(fn Attack)