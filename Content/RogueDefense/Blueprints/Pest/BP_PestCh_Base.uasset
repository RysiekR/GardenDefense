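; Base pest character for RogueDefense that seeks out a plant, damages it once, then destroys itself.
; On spawn it sets its widget bug image, picks a random BP_Plant_Base and paths to it through its AIController.
; Tick polls for idle movement, then sphere-traces to confirm the target before attacking, retargeting with a Niagara effect if other hits exclude it.
; Debug prints, trace drawing and unused right-side targeting logic remain.
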(event Custom|CheckIfHaveAI
  (Utilities|IsValid (AI|GetAIController self)
    (:Is%20Valid
      (Development|PrintString "Have ai controller"))
    (:Is%20Not%20Valid
      (Development|PrintString "dont have ai controller"))))

(event EventBeginPlay
  (bind _aswbp_pest (Utilities|Casting|CastToWBP_Pest (UserInterface|GetWidget (Variables|Default|GetWidget))))
  (Default|ChangeImage _aswbp_pest "/Game/RogueDefense/Downloads/Visuals/bug/Bug0.Bug0")
  (CallFunction|ChooseTarget)
  (CallFunction|GoTowardsTarget))

(event EventTick
  (params (DeltaSeconds :type Float%20%28single-precision%29))
  (bind _capsulecomponent (Variables|Collision|GetCapsuleComponent))
  (bind _returnvalue (Transformation|GetWorldLocation _capsulecomponent))
  (if (> (Actor|GetGameTimeSinceCreation self) 0.1)
    (switch Utilities|FlowControl|Switch|SwitchonEPathFollowingStatus (Class|AIController|GetMoveStatus (AI|GetAIController self))
      (:Idle
        (bind _outhits (Collision|MultiSphereTraceByChannel _returnvalue _returnvalue 2e+02 "TraceTypeQuery1" false 0 "ForDuration"))
        (bind (_array_element _array_index) (Utilities|Array|ForEachLoopwithBreak _outhits :!label _label)
          (:LoopBody
            (if (== (.HitActor (Collision|BreakHitResult _array_element)) (Variables|Default|GetCurrentTarget))
              (Development|PrintString "at plant location")
              (bind _asbp_plant_base (Utilities|Casting|CastToBP_Plant_Base (.HitActor (Collision|BreakHitResult _array_element))))
              (CallFunction|Attack _asbp_plant_base)
              (goto _label Break)
              (elif (== (+ _array_index 1) (Utilities|Array|Length _outhits))
                (CallFunction|ChooseTarget)
                (CallFunction|GoTowardsTarget)
                (Niagara|SpawnSystematLocation "/Game/RogueDefense/Blueprints/NewNiagaraSystem1.NewNiagaraSystem1" (.location (Transformation|GetWorldTransform (Variables|Collision|GetCapsuleComponent))) "0, 0, 0" "10.000000,10.000000,10.000000")))))))))

(fn ConstructionScript)

(fn ChooseTarget
  (bind _outactors (Actor|GetAllActorsOfClass "/Game/RogueDefense/Blueprints/Plant/Base/BP_Plant_Base.BP_Plant_Base_C"))
  (Variables|Default|SetCurrentTarget (.OutItem (Utilities|Array|Random _outactors))))

(fn GoTowardsTarget
  (bind _asaicontroller (Utilities|Casting|CastToAIController (Pawn|GetController)))
  (bind _returnvalue (AI|Navigation|MovetoActor _asaicontroller (Variables|Default|GetCurrentTarget) 1e+02 true true true 0))
  (switch Utilities|FlowControl|Switch|SwitchonEPathFollowingRequestResult _returnvalue
    (:Failed
      (Development|PrintString "Failed pathing"))
    (:AlreadyAtGoal
      (Development|PrintString "already at goal path"))
    (:RequestSuccessful
      (Development|PrintString "path found... going"))))

(fn Attack
  (params (Plant :type BP%20Plant%20Base%20Object%20Reference))
  (Default|Damage Plant (Variables|Default|GetAttackValue))
  (CallFunction|GoAway false))

(fn GoAway
  (params (Reason%28KilledByPlant?%29 :type Boolean))
  (bind _currenttarget (Variables|Default|GetCurrentTarget))
  (if Reason%28KilledByPlant?%29
    (Default|CallOnKill _currenttarget _currenttarget))
  (Actor|DestroyActor))