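; Touch-draggable actor for placing plants on grid locks in mobile RogueDefense, apparently a parent of BP_Plant_Base.
; Touch lifts the cube and widget and binds PC_Mobile move/stop events; screen deltas, scaled by screen height, move a Finger component that highlights the nearest unoccupied BP_GridLockPosition.
; Release lerps the root onto that grid, marks it occupied, has GM_Mobile update plant ranges, then lowers the visuals.
; GetPlantsInRange sphere-traces tagged neighbours for PlantPlacement.
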(event Custom|OnInputTouchBegin_Event
  (params (FingerIndex :type ETouchIndex%20Enum :default "Touch1") (TouchedActor :type Actor%20Object%20Reference))
  (Variables|Default|SetTouching true)
  (bind _aspc_mobile (Utilities|Casting|CastToPC_Mobile (Game|GetPlayerController 0)))
  (EventDispatchers|BindEventtoTouchMove _aspc_mobile (EventDispatchers|CreateEvent :!event Custom|MoveMe))
  (EventDispatchers|BindEventtoStopTouching _aspc_mobile (EventDispatchers|CreateEvent :!event Custom|StopTouch))
  (CallFunction|UpDownAnimation true))

(event Custom|StopTouch
  (Variables|Default|SetTouching false)
  (Variables|Default|SetPreviousLocation "0, 0, 0")
  (bind _aspc_mobile (Utilities|Casting|CastToPC_Mobile (Game|GetPlayerController 0)))
  (EventDispatchers|UnbindEventfromTouchMove _aspc_mobile (EventDispatchers|CreateEvent :!event Custom|MoveMe))
  (EventDispatchers|UnbindEventfromStopTouching _aspc_mobile (EventDispatchers|CreateEvent :!event Custom|StopTouch))
  (Transformation|SetRelativeLocation (Variables|Default|GetFinger) "0, 0, 0" false false)
  (bind (_direction _newtrack_0 _highttrack) (Timeline|Timeline PlayFromStart)
    (:Update
      (bind _cachedgrid (Variables|Default|GetCachedGrid)
        (:then
          (Transformation|SetWorldLocation (Variables|Default|GetDefaultSceneRoot) (Math|Vector|MakeVector (.X (Math|Vector|BreakVector (Math|Vector|Lerp(Vector) (Transformation|GetWorldLocation (Variables|Default|GetDefaultSceneRoot)) (Transformation|GetWorldLocation (Variables|/Game/RogueDefense/Blueprints/GridLockPosition/BP_GridLockPosition.BP_GridLockPosition_C|GetDefaultSceneRoot _cachedgrid)) _newtrack_0))) (.Y (Math|Vector|BreakVector (Math|Vector|Lerp(Vector) (Transformation|GetWorldLocation (Variables|Default|GetDefaultSceneRoot)) (Transformation|GetWorldLocation (Variables|/Game/RogueDefense/Blueprints/GridLockPosition/BP_GridLockPosition.BP_GridLockPosition_C|GetDefaultSceneRoot _cachedgrid)) _newtrack_0))) (.Z (Math|Vector|BreakVector (Math|Vector|Lerp(Vector) (Transformation|GetWorldLocation (Variables|Default|GetDefaultSceneRoot)) (Transformation|GetWorldLocation (Variables|/Game/RogueDefense/Blueprints/GridLockPosition/BP_GridLockPosition.BP_GridLockPosition_C|GetDefaultSceneRoot _cachedgrid)) _newtrack_0)))) false false)
          (Default|SetOccupied (Variables|Default|GetCachedGrid) true))
        (:else)))
    (:Finished
      (bind _asgm_mobile (Utilities|Casting|CastToGM_Mobile (Game|GetGameMode)))
      (Default|UpdatePlantsinRange _asgm_mobile)
      (CallFunction|UpDownAnimation false))))

(event Custom|MoveMe
  (params (FingerLocation :type Vector))
  (bind _finger (Variables|Default|GetFinger))
  (bind _returnvalue (Transformation|GetWorldLocation _finger))
  (bind _cachedgrid (Variables|Default|GetCachedGrid)
    (:then
      (Default|SetOccupied _cachedgrid false))
    (:else
      (Development|PrintString "grid cache not valid, do we even care ?")))
  (if (Class|KismetMathLibrary|EqualExactlyVectorVector (Variables|Default|GetPreviousLocation) "0, 0, 0")
    (Variables|Default|SetPreviousLocation FingerLocation)
    (else
      (bind (_x_outputpin _y_outputpin2 _z_outputpin3) (CallFunction|GetDeltaMovetoWorld FingerLocation))
      (Class|SceneComponent|AddWorldTransform (Variables|Default|GetFinger) (Math|Transform|MakeTransform (Math|Vector|MakeVector _x_outputpin _y_outputpin2 _z_outputpin3) "0, 0, 0" "1.000000,1.000000,1.000000") false false)
      (Variables|Default|SetPreviousLocation FingerLocation)
      (Variables|Default|SetLastFingerPlace _returnvalue)
      (bind _gridlocation (CallFunction|FindClosestGridLock _returnvalue))
      (CallFunction|HighlightGridF _gridlocation))))

(event Custom|UpDownAnimation
  (params (Up? :type Boolean))
  (bind _returnvalue (Math|Float|MakeLiteralFloat 1e+01))
  (if Up?
    (bind (_direction _newtrack_0) (Timeline|Timeline_0 Play)
      (:Update
        (if (Utilities|Enum|Equal(Enum) _direction "Forward")
          (Transformation|AddRelativeLocation (Variables|Default|GetWidget) (Math|Vector|MakeVector 0.0 0.0 (* _newtrack_0 _returnvalue)) false false)
          (else
            (Transformation|AddRelativeLocation (Variables|Default|GetWidget) (Math|Vector|MakeVector 0.0 0.0 (* _newtrack_0 _returnvalue -1.0)) false false))))
      (:Finished
        (if (not (Utilities|Enum|Equal(Enum) _direction "Forward"))
          (Transformation|SetRelativeLocation (Variables|Default|GetCube) (Variables|Default|GetResetLocationCube) false false)
          (Transformation|SetRelativeLocation (Variables|Default|GetWidget) (Variables|Default|GetResetLocationWidget) false false))))
    (else
      (Timeline|Timeline_0 Reverse))))

(event EventBeginPlay
  ;[0 1 0.1] Start
  (EventDispatchers|AssignOnInputTouchBegin (delegate Custom|OnInputTouchBegin_Event))
  (Variables|Default|SetResetLocationCube (Variables|/Script/Engine.SceneComponent|GetRelativeLocation (Variables|Default|GetCube)))
  (Variables|Default|SetResetLocationWidget (Variables|/Script/Engine.SceneComponent|GetRelativeLocation (Variables|Default|GetWidget))))

(fn ConstructionScript)

(fn GetDeltaMovetoWorld
  (params (FingerLocation :type Vector))
  (bind _previouslocation (Variables|Default|GetPreviousLocation))
  (bind _returnvalue (- _previouslocation FingerLocation))
  (bind _returnvalue_2 (* _returnvalue 5.0 1.0))
  (return (* (.x _returnvalue_2) 1.2) (* (.y _returnvalue_2) (Math|Float|MapRangeClamped (.Y (Math|Vector|BreakVector FingerLocation)) 0.0 1e+04 2.5 0.8)) (.z _returnvalue_2)))

(fn FindClosestGridLock
  (params (InLocation :type Vector))
  (LocalVariables|SetTempDistance 9999999.0)
  (LocalVariables|SetTempClosest 0)
  (bind _outactors (Actor|GetAllActorsOfClass "/Game/RogueDefense/Blueprints/GridLockPosition/BP_GridLockPosition.BP_GridLockPosition_C"))
  (for _array_element _outactors
    (if (and (< (Math|Vector|Distance(Vector) (Transformation|GetWorldLocation (Variables|/Game/RogueDefense/Blueprints/GridLockPosition/BP_GridLockPosition.BP_GridLockPosition_C|GetDefaultSceneRoot _array_element)) InLocation) (LocalVariables|GetTempDistance)) (not (Variables|/Game/RogueDefense/Blueprints/GridLockPosition/BP_GridLockPosition.BP_GridLockPosition_C|GetOccupied? _array_element)))
      (LocalVariables|SetTempClosest _array_element)
      (LocalVariables|SetTempDistance (Math|Vector|Distance(Vector) (Transformation|GetWorldLocation (Variables|/Game/RogueDefense/Blueprints/GridLockPosition/BP_GridLockPosition.BP_GridLockPosition_C|GetDefaultSceneRoot _array_element)) InLocation))))
  (return (LocalVariables|GetTempClosest)))

(fn GetPlantsinRange
  (bind _defaultsceneroot (Variables|Default|GetDefaultSceneRoot))
  (bind _returnvalue (Transformation|GetWorldLocation _defaultsceneroot))
  (bind _asbp_plant_base (Utilities|Casting|CastToBP_Plant_Base self))
  (bind _outhits (Collision|MultiSphereTraceByChannel _returnvalue _returnvalue (Variables|/Game/RogueDefense/Blueprints/Plant/Base/BP_Plant_Base.BP_Plant_Base_C|GetRangeOfInfluence _asbp_plant_base) "TraceTypeQuery1" false 0 "ForDuration"))
  (bind _array_element (Utilities|Array|ForEachLoopwithBreak _outhits)
    (:LoopBody
      (if (Components|ComponentHasTag (.HitComponent (Collision|BreakHitResult _array_element)) "RootToCheckPlantPlacement")
        (bind _asbp_plant_base_2 (Utilities|Casting|CastToBP_Plant_Base (.HitActor (Collision|BreakHitResult _array_element))))
        (Utilities|Array|AddUnique (LocalVariables|GetTempArray) _asbp_plant_base_2)))
    (:Completed
      (Default|PlantPlacement _asbp_plant_base (LocalVariables|GetTempArray)))))

(fn HighlightGridF
  (params (NewGrid :type BP%20Grid%20Lock%20Position%20Object%20Reference))
  (Utilities|IsValid (Variables|Default|GetCachedGrid)
    (:Is%20Valid
      (if (not (== NewGrid (Variables|Default|GetCachedGrid)))
        (Utilities|IsValid NewGrid
          (:Is%20Valid
            (Default|UnHighlight (Variables|Default|GetCachedGrid))
            (bind _output_get (Variables|Default|SetCachedGrid NewGrid))
            (Default|Highlight _output_get))
          (:Is%20Not%20Valid
            (Default|UnHighlight (Variables|Default|GetCachedGrid))
            (Variables|Default|SetCachedGrid 0)))))
    (:Is%20Not%20Valid
      (Utilities|IsValid NewGrid
        (:Is%20Valid
          (bind _output_get_2 (Variables|Default|SetCachedGrid NewGrid))
          (Default|Highlight _output_get_2))))))