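; BP_Bench is the bench actor in RogueDefense, providing a row of lock positions as slots.
; On BeginPlay, Init copies Slots into FreeSlots and spawns one BP_GridLockPosition per slot.
; Each is spaced at a fixed world X offset from the FirstSlot component, given a fixed yaw or axis rotation, and stored in BenchGrid.
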(event Custom|Init
  (bind _firstslot (Variables|Default|GetFirstSlot))
  (bind _returnvalue (Transformation|GetWorldLocation _firstslot))
  (bind _output_get (Variables|Default|SetFreeSlots (Variables|Default|GetSlots)))
  (for _index (range 0 (- _output_get 1))
    (bind _returnvalue_2 (Game|SpawnActorfromClass "/Game/RogueDefense/Blueprints/GridLockPosition/BP_GridLockPosition.BP_GridLockPosition_C" (Math|Transform|MakeTransform "0, 0, 0" "0, 0, 0" "1.000000,1.000000,1.000000") "AlwaysSpawn" "MultiplyWithRoot" 0 0))
    (Transformation|SetWorldLocation (Variables|/Game/RogueDefense/Blueprints/GridLockPosition/BP_GridLockPosition.BP_GridLockPosition_C|GetDefaultSceneRoot _returnvalue_2) (Math|Vector|MakeVector (+ (.x _returnvalue) (* _index 800)) (.y _returnvalue) (.z _returnvalue)) false false)
    (Transformation|SetWorldRotation (Variables|/Game/RogueDefense/Blueprints/GridLockPosition/BP_GridLockPosition.BP_GridLockPosition_C|GetDefaultSceneRoot _returnvalue_2) "0.000000,-90.000000,0.000000" false false)
    (Utilities|Array|AddUnique (Variables|Default|GetBenchGrid) _returnvalue_2)))

(event EventBeginPlay
  (CallFunction|Init))

(fn ConstructionScript)