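; BP_Pot_Base is the base Blueprint for pots, layered on a parent class that supplies grid-lock lookup.
; On BeginPlay it runs the parent logic, then passes PotImage to its WBP_PlantDisplayWidget to set the displayed image.
; It overrides FindClosestGridLock to call the parent with the type fixed to "Pot", ignoring the PlantOrPot argument it receives.
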(event EventBeginPlay
  (|CallParentFunction)
  (bind _aswbp_plant_display_widget (Utilities|Casting|CastToWBP_PlantDisplayWidget (UserInterface|GetWidget (Variables|Default|GetWidget))))
  (Default|ChangeImage _aswbp_plant_display_widget (Variables|Default|GetPotImage)))

(fn ConstructionScript
  (|CallParentFunction))

(fn FindClosestGridLock
  (params (InLocation :type Vector :default "0, 0, 0") (PlantOrPot :type Name :default "None"))
  (bind _gridlocation (|CallParentFunction InLocation "Pot"))
  (return _gridlocation))