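; Cherry plant for RogueDefense that boosts plants on the field through overrides of the sell, growth and death effects.
; When the parent effect succeeds, selling refills the amount and growth doubles the max amount on three random picks among other plants.
; Death adds each plant's base value to every plant.
; Random is evaluated separately for read and write, so values can come from a different plant.
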(event EventBeginPlay
  (|CallParentFunction) ; This node is disabled and will not be called.\nDrag off pins to build functionality.
)

(event Collision|EventActorBeginOverlap
  (params (OtherActor :type Actor%20Object%20Reference)))

(event EventTick
  (params (DeltaSeconds :type Float%20%28single-precision%29)))

(fn ConstructionScript
  (|CallParentFunction))

(fn SellEEF
  (params (Performer :type Actor%20Object%20Reference))
  (bind _canchildperform (|CallParentFunction Performer))
  (if _canchildperform
    (bind _outactors (Actor|GetAllActorsOfClass "/Game/RogueDefense/Blueprints/Plant/Base/BP_Plant_Base.BP_Plant_Base_C"))
    (Utilities|Array|RemoveItem _outactors self)
    (for _index (range 0 2)
      (Utilities|Struct|SetmembersinSTRUCT_PlantAmmount (Variables|/Game/RogueDefense/Blueprints/Plant/Base/BP_Plant_Base.BP_Plant_Base_C|GetAmmount (.OutItem (Utilities|Array|Random _outactors))) (.MaxAmmount (Utilities|Struct|BreakSTRUCT_PlantAmmount (Variables|/Game/RogueDefense/Blueprints/Plant/Base/BP_Plant_Base.BP_Plant_Base_C|GetAmmount (.OutItem (Utilities|Array|Random _outactors)))))))))

(fn GrowthEEF
  (params (NewGrowthStage :type ENUM_PlantGrowthStage%20Enum :default "NewEnumerator0") (Performer :type Actor%20Object%20Reference))
  (bind _canchildperform (|CallParentFunction NewGrowthStage Performer))
  (if _canchildperform
    (bind _outactors (Actor|GetAllActorsOfClass "/Game/RogueDefense/Blueprints/Plant/Base/BP_Plant_Base.BP_Plant_Base_C"))
    (Utilities|Array|RemoveItem _outactors self)
    (for _index (range 0 2)
      (Utilities|Struct|SetmembersinSTRUCT_PlantAmmount (Variables|/Game/RogueDefense/Blueprints/Plant/Base/BP_Plant_Base.BP_Plant_Base_C|GetAmmount (.OutItem (Utilities|Array|Random _outactors))) (* (.MaxAmmount (Utilities|Struct|BreakSTRUCT_PlantAmmount (Variables|/Game/RogueDefense/Blueprints/Plant/Base/BP_Plant_Base.BP_Plant_Base_C|GetAmmount (.OutItem (Utilities|Array|Random _outactors))))) 2)))))

(fn DeathEEF
  (params (Performer :type Actor%20Object%20Reference))
  (bind _canchildperform (|CallParentFunction Performer))
  (if _canchildperform
    (bind _outactors (Actor|GetAllActorsOfClass "/Game/RogueDefense/Blueprints/Plant/Base/BP_Plant_Base.BP_Plant_Base_C"))
    (for _array_element _outactors
      (Default|AddValueF _array_element (.BaseValue (Utilities|Struct|BreakSTRUCT_PlantValue (Variables|/Game/RogueDefense/Blueprints/Plant/Base/BP_Plant_Base.BP_Plant_Base_C|GetValue _array_element)))))))