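; Base plant actor for a roguelike defense game, with growth and health stages, temporary HP, selling and an info widget.
; It loads stats from DT_PlantInfo, occupies a grid cell and gains or loses stat bonuses from nearby pots.
; Pollination spawns same-species, crossbred or occasional random plants on free cells.
; Dispatchers feed EEF hook functions that always accept self-triggered events but accept other performers' only once, via flags.
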(event Custom|Pollinate
  (if (Utilities|Enum|Equal(Enum) (Variables|Default|GetGrowthStage) "NewEnumerator3")
    (bind _chosenplants (CallFunction|ChoosePlantstoPollinate))
    (CallFunction|PollinateF _chosenplants)))

(event Custom|ApplyPotToThisPlant
  (params (ValueToAdd :type Float%20%28double-precision%29) (AmountToAdd :type Integer) (MaxAmountToAdd :type Integer))
  (bind _value (Variables|Default|GetValue))
  (bind _ammount (Variables|Default|GetAmmount))
  (bind _ammount_2 (Variables|Default|GetAmmount))
  (if (not (Variables|PotChanges|GetPotApplied))
    (Variables|PotChanges|SetPotAddValue ValueToAdd)
    (Variables|PotChanges|SetPot%20Amount%20to%20Add AmountToAdd)
    (Variables|PotChanges|SetPot%20Max%20Amount%20to%20Add MaxAmountToAdd)
    (Utilities|Struct|SetmembersinSTRUCT_PlantValue _value (+ ValueToAdd (.Value (Utilities|Struct|BreakSTRUCT_PlantValue _value))))
    (Utilities|Struct|SetmembersinSTRUCT_PlantAmmount _ammount (+ AmountToAdd (.Ammount (Utilities|Struct|BreakSTRUCT_PlantAmmount _ammount))))
    (Utilities|Struct|SetmembersinSTRUCT_PlantAmmount _ammount_2 (+ MaxAmountToAdd (.MaxAmmount (Utilities|Struct|BreakSTRUCT_PlantAmmount _ammount_2))))
    (Variables|PotChanges|SetPotApplied true)
    (Default|CallUpdateUI)))

(event Custom|UnApplyLastPot
  (bind _value (Variables|Default|GetValue))
  (bind _ammount (Variables|Default|GetAmmount))
  (bind _ammount_2 (Variables|Default|GetAmmount))
  (if (Variables|PotChanges|GetPotApplied)
    (Utilities|Struct|SetmembersinSTRUCT_PlantValue _value (Math|Float|Max(Float) (- (.Value (Utilities|Struct|BreakSTRUCT_PlantValue _value)) (Variables|PotChanges|GetPotAddValue)) 1.0))
    (Utilities|Struct|SetmembersinSTRUCT_PlantAmmount _ammount_2 (Math|Integer|Max(Integer) (- (.Ammount (Utilities|Struct|BreakSTRUCT_PlantAmmount _ammount_2)) (Variables|PotChanges|GetPot%20Amount%20to%20Add)) 1))
    (Utilities|Struct|SetmembersinSTRUCT_PlantAmmount _ammount (Math|Integer|Max(Integer) (- (.MaxAmmount (Utilities|Struct|BreakSTRUCT_PlantAmmount _ammount)) (Variables|PotChanges|GetPot%20Max%20Amount%20to%20Add)) 1))
    (Variables|PotChanges|SetPotApplied false)
    (Default|CallUpdateUI)))

(event Custom|NowApplyPot_Event
  (bind _cube (Variables|Default|GetCube))
  (bind _returnvalue (Transformation|GetWorldLocation _cube))
  (bind _outhits (Collision|MultiSphereTraceByChannel _returnvalue _returnvalue 1e+02 "TraceTypeQuery1" false 0 "None" true "(R=1.000000,G=0.000000,B=0.617640,A=1.000000)"))
  (bind _array_element (Utilities|Array|ForEachLoopwithBreak _outhits :!label _label)
    (:LoopBody
      (bind _asbp_pot_base (Utilities|Casting|CastToBP_Pot_Base (.HitActor (Collision|BreakHitResult _array_element))))
      (bind (_plantvalueadd _ammountadd _maxammountadd) (Default|GetPlantModifiers _asbp_pot_base))
      (CallFunction|ApplyPottoThisPlant _plantvalueadd _ammountadd _maxammountadd)
      (Development|PrintString "Applied pot to this plant")
      (goto _label Break))))

(event Custom|NowUnApplyPot_Event
  (CallFunction|UnApplyLastPot))

(event Custom|UpdateUI_Event
  (CallFunction|CloseInfoDisplay)
  (CallFunction|DisplayInfo))

(event EventBeginPlay
  ;[0 1 0.1 0.5] BeginPlay
  (|CallParentFunction)
  (CallFunction|Init)
  (CallFunction|GetPlantsinRange)
  (CallFunction|EventEffectBinder)
  (Utilities|FlowControl|Sequence
    (:then_0
      (EventDispatchers|AssignNowApplyPot (delegate Custom|NowApplyPot_Event))
      (EventDispatchers|AssignNowUnApplyPot (delegate Custom|NowUnApplyPot_Event))
      (EventDispatchers|BindEventtoUpdateUI (delegate Custom|UpdateUI_Event)))))

(event EventEndPlay
  (params (EndPlayReason :type EEndPlayReason%20Enum :default "Destroyed"))
  (CallFunction|CloseInfoDisplay)
  (CallFunction|EventEffectUnbinder)
  (bind _asgm_mobile (Utilities|Casting|CastToGM_Mobile (Game|GetGameMode)))
  (Default|UpdatePlantsinRange _asgm_mobile)
  (bind _cachedgrid (Variables|Default|GetCachedGrid)
    (:then
      (Default|SetOccupied _cachedgrid false)
      (Default|IDiedChangeTarget _asgm_mobile self))
    (:else)))

(event Custom|EventEffectBinder
  ;[0.15 0.15 0.15 0.5] Bind / Unbind Events
  (EventDispatchers|BindEventtoOnGrowthStageChange (EventDispatchers|CreateEvent :!event Custom|OnGrowthStageChange_Event))
  (EventDispatchers|BindEventtoOnDeath (EventDispatchers|CreateEvent :!event Custom|OnDeath_Event))
  (EventDispatchers|BindEventtoOnPollinate (EventDispatchers|CreateEvent :!event Custom|OnPollinate_Event))
  (EventDispatchers|BindEventtoOnKill (EventDispatchers|CreateEvent :!event Custom|OnKill_Event))
  (EventDispatchers|BindEventtoOnHealthChange (EventDispatchers|CreateEvent :!event Custom|OnHealthChange_Event))
  (EventDispatchers|BindEventtoOnSell (EventDispatchers|CreateEvent :!event Custom|OnSell_Event)))

(event Custom|EventEffectUnbinder
  ;[0.15 0.15 0.15 0.5] Bind / Unbind Events
  (EventDispatchers|UnbindallEventsfromOnGrowthStageChange)
  (EventDispatchers|UnbindallEventsfromOnDeath)
  (EventDispatchers|UnbindallEventsfromOnPollinate)
  (EventDispatchers|UnbindallEventsfromOnKill)
  (EventDispatchers|UnbindallEventsfromOnHealthChange)
  (EventDispatchers|UnbindallEventsfromOnSell))

(event Custom|OnGrowthStageChange_Event
  (params (NewGrowthStage :type ENUM_PlantGrowthStage%20Enum :default "NewEnumerator0") (Performer :type Actor%20Object%20Reference))
  (EventEffectFunction|GrowthEEF NewGrowthStage Performer))

(event Custom|OnPollinate_Event
  (params (Performer :type Actor%20Object%20Reference))
  (EventEffectFunction|PollinateEEF Performer))

(event Custom|OnKill_Event
  (params (Performer :type Actor%20Object%20Reference))
  (EventEffectFunction|KillEEF Performer))

(event Custom|OnHealthChange_Event
  (params (NewHealth :type ENUM_HealthStage%20Enum :default "NewEnumerator0") (Performer :type Actor%20Object%20Reference))
  (EventEffectFunction|HealthChangeEEF NewHealth Performer))

(event Custom|OnSell_Event
  (params (Performer :type Actor%20Object%20Reference))
  (EventEffectFunction|SellEEF Performer))

(event Custom|OnDeath_Event
  (params (Performer :type Actor%20Object%20Reference))
  (EventEffectFunction|DeathEEF Performer)
  (if (== Performer self)
    (Development|PrintString "Eventgraph goodbye")
    (bind _cachedgrid (Variables|Default|GetCachedGrid)
      (:then
        (Default|SetOccupied _cachedgrid false))
      (:else
        _))
    (Actor|DestroyActor)))

(event Custom|DisplayInfo
  (bind _asgm_mobile (Utilities|Casting|CastToGM_Mobile (Game|GetGameMode)))
  (Default|ClosePlantInfo _asgm_mobile)
  (bind _returnvalue (UserInterface|CreateWidget "/Game/RogueDefense/Blueprints/Plant/Base/WBP_InfoPlantDisplay.WBP_InfoPlantDisplay_C" 0 (Variables|Default|GetName) self))
  (bind _output_get (Variables|Default|SetWidgetInfo _returnvalue))
  (UserInterface|Viewport|AddtoViewport _output_get 0))

(event Custom|CloseInfoDisplay
  (bind _widgetinfo (Variables|Default|GetWidgetInfo)
    (:then
      (Widget|RemovefromParent _widgetinfo)
      (Variables|Default|SetWidgetInfo 0))
    (:else)))

(fn ConstructionScript
  (|CallParentFunction))

(fn AddTempHP
  (params (Type :type ENUM_TempHealthName%20Enum :default "NewEnumerator0") (Ammount :type Integer))
  (bind _temphealthbuff (Variables|Default|GetTempHealthBuff))
  (bind (_value _returnvalue) (Utilities|Map|Find _temphealthbuff Type))
  (if _returnvalue
    (bind _returnvalue_2 (Class|KismetSystemLibrary|MakeLiteralInteger _value))
    (Utilities|Map|Remove (Variables|Default|GetTempHealthBuff) Type)
    (Utilities|Map|Add (Variables|Default|GetTempHealthBuff) Type (+ _returnvalue_2 Ammount))
    (else
      (Utilities|Map|Add (Variables|Default|GetTempHealthBuff) Type Ammount))))

(fn TestPrint
  (bind _keys (Utilities|Map|Keys (Variables|Default|GetTempHealthBuff)))
  (for _array_element _keys
    (Development|PrintText (Utilities|Text|FormatText "Type:{a}, Ammount:{b}" (|GenerictoText _array_element) (.Value (Utilities|Map|Find (Variables|Default|GetTempHealthBuff) _array_element))))))

(fn RemoveTempHp
  (params (Ammount :type Integer))
  (LocalVariables|SetAmmountLeft Ammount)
  (while (and (> (LocalVariables|GetAmmountLeft) 0) (Utilities|Map|IsNotEmpty (Variables|Default|GetTempHealthBuff)))
    (bind _keys (Utilities|Map|Keys (Variables|Default|GetTempHealthBuff)))
    ;[0.15 0.15 0.15 0.5] exec pins to cache values
    (bind _outitem (Utilities|Array|Random _keys))
    (bind _value (Utilities|Map|Find (Variables|Default|GetTempHealthBuff) _outitem))
    (if (== _value (LocalVariables|GetAmmountLeft))
      ;[0.15 0.15 0.15 0.5] Przypadek dmg = temphp
      (Utilities|Map|Remove (Variables|Default|GetTempHealthBuff) _outitem)
      (LocalVariables|SetAmmountLeft 0)
      (elif (> _value (LocalVariables|GetAmmountLeft))
        ;[0.15 0.15 0.15 0.5] Przypadek ze zostało jeszcze tempHp
        (Utilities|Map|Remove (Variables|Default|GetTempHealthBuff) _outitem)
        (Utilities|Map|Add (Variables|Default|GetTempHealthBuff) _outitem (- _value (LocalVariables|GetAmmountLeft)))
        (LocalVariables|SetAmmountLeft 0)
        (else
          ;[0.15 0.15 0.15 0.5] Przypadek dmg wiekszy niz temp hp
          (Utilities|Map|Remove (Variables|Default|GetTempHealthBuff) _outitem)
          (LocalVariables|SetAmmountLeft (- (LocalVariables|GetAmmountLeft) _value))))))
  (Development|PrintText (Utilities|Text|FormatText "damage left:{a}" (LocalVariables|GetAmmountLeft)))
  (return (LocalVariables|GetAmmountLeft)))

(fn PollinateF
  (params (ChooseFrom :type Array%20of%20BP%20Plant%20Base%20Object%20References))
  (bind _onlycrosspollination (CallFunction|LimitArraytoCrossPollination ChooseFrom))
  (if (> (Utilities|Array|Length _onlycrosspollination) 0)
    (bind _gridlocation (CallFunction|FindClosestGridLock (Transformation|GetWorldLocation (Variables|Default|GetDefaultSceneRoot)) "None"))
    (Utilities|IsValid _gridlocation
      (:Is%20Valid
        (bind _output_get (LocalVariables|SetTempGrid _gridlocation))
        (LocalVariables|SetTempSpawnTransform (Transformation|GetActorTransform _output_get))
        ;[0.15 0.15 0.15 0.5] Chosen
        (bind _returnvalue (Utilities|GetDataTableRow "/Game/RogueDefense/Blueprints/Plant/DT_PlantInfo.DT_PlantInfo" (Variables|Default|GetName))
          (:then
            (Development|PrintText (Utilities|Text|FormatText "this class:{a} with {b} , from:{c}" (Variables|Default|GetName) (Variables|BP_Plant_Base_C|GetName (.OutItem (Utilities|Array|Random _onlycrosspollination))) (Utilities|Array|Length _onlycrosspollination)) true true "(R=0.000000,G=0.660000,B=1.000000,A=1.000000)" 2e+01)
            (if (== (Utilities|GetClass (.OutItem (Utilities|Array|Random _onlycrosspollination))) (.Plant (Utilities|Struct|BreakSTRUCT_PlantInfo _returnvalue)))
              (Development|PrintString "same plant" true true "(R=1.000000,G=0.582529,B=0.000000,A=1.000000)" 2e+01)
              ;;[0.15 0.15 0.15 0.5] same plant
              (bind _returnvalue_2 (Game|SpawnActorfromClass (.Plant (Utilities|Struct|BreakSTRUCT_PlantInfo _returnvalue)) (LocalVariables|GetTempSpawnTransform) "Undefined" "MultiplyWithRoot" 0 (.Name (Utilities|Struct|BreakSTRUCT_PlantInfo _returnvalue)) 0))
              (bind _output_get_2 (Variables|/Game/RogueDefense/Blueprints/BP_TouchTest.BP_TouchTest_C|SetCachedGrid _returnvalue_2 (LocalVariables|GetTempGrid)))
              (Default|SetOccupied _output_get_2 true)
              (else
                ;;[0.15 0.15 0.15 0.5] Cross pollination
                (if (.ReturnValue (Utilities|Map|Find (.CrossPollinationwithproduce (Utilities|Struct|BreakSTRUCT_PlantInfo _returnvalue)) (Utilities|GetClass (.OutItem (Utilities|Array|Random _onlycrosspollination)))))
                  (Development|PrintString "cross pollination" true true "(R=1.000000,G=0.466937,B=0.000000,A=1.000000)" 2e+01)
                  (bind _returnvalue_3 (Utilities|GetDataTableRow "/Game/RogueDefense/Blueprints/Plant/DT_PlantInfo.DT_PlantInfo" (.Value (Utilities|Map|Find (.CrossPollinationwithproduce (Utilities|Struct|BreakSTRUCT_PlantInfo _returnvalue)) (Utilities|GetClass (.OutItem (Utilities|Array|Random _onlycrosspollination))))))
                    (:then
                      (bind _returnvalue_4 (Game|SpawnActorfromClass (.Plant (Utilities|Struct|BreakSTRUCT_PlantInfo _returnvalue_3)) (LocalVariables|GetTempSpawnTransform) "Undefined" "MultiplyWithRoot" 0 (.Name (Utilities|Struct|BreakSTRUCT_PlantInfo _returnvalue_3)) 0))
                      (bind _output_get_3 (Variables|/Game/RogueDefense/Blueprints/BP_TouchTest.BP_TouchTest_C|SetCachedGrid _returnvalue_4 (LocalVariables|GetTempGrid)))
                      (Default|SetOccupied _output_get_3 true)))
                  (else
                    ;;[0.15 0.15 0.15 0.5] Pitty Random seed
                    (bind _outrownames (DataTable|GetDataTableRowNames "/Game/RogueDefense/Blueprints/Plant/DT_PlantInfo.DT_PlantInfo"))
                    (bind _returnvalue_5 (Utilities|GetDataTableRow "/Game/RogueDefense/Blueprints/Plant/DT_PlantInfo.DT_PlantInfo" (.OutItem (Utilities|Array|Random _outrownames)))
                      (:then
                        (if (and (<= (.Tier (Utilities|Struct|BreakSTRUCT_PlantInfo _returnvalue_5)) (.Tier (Utilities|Struct|BreakSTRUCT_PlantInfo _returnvalue))) (> (Math|Random|RandomIntegerinRange 0 100) 90))
                          (bind _returnvalue_6 (Game|SpawnActorfromClass (.Plant (Utilities|Struct|BreakSTRUCT_PlantInfo _returnvalue_5)) (LocalVariables|GetTempSpawnTransform) "Undefined" "MultiplyWithRoot" 0 (.Name (Utilities|Struct|BreakSTRUCT_PlantInfo _returnvalue_5)) 0))
                          (bind _output_get_4 (Variables|/Game/RogueDefense/Blueprints/BP_TouchTest.BP_TouchTest_C|SetCachedGrid _returnvalue_6 (LocalVariables|GetTempGrid)))
                          (Default|SetOccupied _output_get_4 true)))))))))))
      (:Is%20Not%20Valid
        (Development|PrintString "no free grid spots")))
    (elif (> (Utilities|Array|Length ChooseFrom) 0)
      (Development|PrintString "implement pitty here."))))

(fn Init
  (Utilities|FlowControl|Sequence
    (:then_0
      (EventDispatchers|BindEventtoDisplayInfoDispatcher (EventDispatchers|CreateEvent :!event Custom|DisplayInfo)))
    (:then_1
      (bind _returnvalue (Utilities|GetDataTableRow "/Game/RogueDefense/Blueprints/Plant/DT_PlantInfo.DT_PlantInfo" (Variables|Default|GetName))
        (:then
          (Utilities|Struct|SetmembersinSTRUCT_PlantValue (Variables|Default|GetValue) (.Value (Utilities|Struct|BreakSTRUCT_PlantInfo _returnvalue)) (.Value (Utilities|Struct|BreakSTRUCT_PlantInfo _returnvalue)))
          (Utilities|Struct|SetmembersinSTRUCT_PlantAmmount (Variables|Default|GetAmmount) (.Ammount (Utilities|Struct|BreakSTRUCT_PlantInfo _returnvalue)) (.Ammount (Utilities|Struct|BreakSTRUCT_PlantInfo _returnvalue)) (.Ammount (Utilities|Struct|BreakSTRUCT_PlantInfo _returnvalue)))
          (Variables|Default|SetPrestigeTier (.Tier (Utilities|Struct|BreakSTRUCT_PlantInfo _returnvalue)))
          (Variables|Default|SetRangeOfInfluence (.RangeOfInfluence (Utilities|Struct|BreakSTRUCT_PlantInfo _returnvalue)))
          ;[0.15 0.15 0.15 0.5] load images?
          (bind _aswbp_plant_display_widget (Utilities|Casting|CastToWBP_PlantDisplayWidget (UserInterface|GetWidget (Variables|Default|GetWidget)))
            (:then
              (Default|ChangeImage _aswbp_plant_display_widget (Utilities|Array|Get(acopy) (Variables|Default|GetImages))))
            (:CastFailed
              (Development|PrintString "fail load img0" true true "(R=1.000000,G=0.141495,B=0.000000,A=1.000000)"))))))))

(fn GrowF
  (if (Utilities|Enum|NotEqual(Enum) (Variables|Default|GetGrowthStage) "NewEnumerator4")
    (bind _result (Math|Integer|IncrementInt (Math|Conversions|ToInteger(Byte) (Variables|Default|GetGrowthStage)))
      (:%20%20
        (bind _output_get (Variables|Default|SetGrowthStage (Utilities|Enum|ByteToEnumENUM_PlantGrowthStage (Math|Conversions|ToByte(Integer) _result))))
        (bind _aswbp_plant_display_widget (Utilities|Casting|CastToWBP_PlantDisplayWidget (UserInterface|GetWidget (Variables|Default|GetWidget))))
        (Default|ChangeImage _aswbp_plant_display_widget (Utilities|Array|Get(acopy) (Variables|Default|GetImages) _result))
        (Default|CallOnGrowthStageChange _output_get self)))
    (else
      (Default|CallOnDeath self))))

(fn Damage
  (params (Amount :type Integer))
  (bind _ammountnotdealt (HPRelated|RemoveTempHp Amount))
  (if (> _ammountnotdealt 0)
    (bind _result (Math|Integer|IncrementInt (Math|Conversions|ToInteger(Byte) (Variables|Default|GetHealth)))
      (:%20%20
        (bind _output_get (Variables|Default|SetHealth (Utilities|Enum|ByteToEnumENUM_HealthStage (Math|Conversions|ToByte(Integer) _result))))
        (switch Utilities|FlowControl|Switch|SwitchonENUM_HealthStage _output_get
          (:NewEnumerator0
            (Default|CallOnHealthChange _output_get self :!label _label))
          (:NewEnumerator1
            (goto _label))
          (:NewEnumerator2
            (goto _label))
          (:NewEnumerator3
            (goto _label))
          (:NewEnumerator4
            (Default|CallOnDeath self)))))))

(fn GrowthEEF
  (params (NewGrowthStage :type ENUM_PlantGrowthStage%20Enum :default "NewEnumerator0") (Performer :type Actor%20Object%20Reference))
  (Utilities|IsValid Performer
    (:Is%20Valid
      (if (== Performer self)
        _
        (else
          (if (Variables|EffectFlag|GetGrowthFlag) :!label _label
            (return false)
            (else
              (Variables|EffectFlag|SetGrowthFlag true))))))
    (:Is%20Not%20Valid
      (goto _label)))
  (return true))

(fn DeathEEF
  (params (Performer :type Actor%20Object%20Reference))
  (Utilities|IsValid Performer
    (:Is%20Valid
      (if (== Performer self)
        _
        (else
          (if (Variables|EffectFlag|GetDeathFlag) :!label _label
            (return false)
            (else
              (Variables|EffectFlag|SetDeathFlag true))))))
    (:Is%20Not%20Valid
      (goto _label)))
  (Development|PrintString "parent goodbye")
  (return true))

(fn PollinateEEF
  (params (Performer :type Actor%20Object%20Reference))
  (if (== Performer self)
    _
    (elif (Variables|EffectFlag|GetPollinateFlag)
      (return false)
      (else
        (Variables|EffectFlag|SetPollinateFlag true))))
  (return true))

(fn KillEEF
  (params (Performer :type Actor%20Object%20Reference))
  (if (== Performer self)
    _
    (elif (Variables|EffectFlag|GetKillFlag)
      (return false)
      (else
        (Variables|EffectFlag|SetKillFlag true))))
  (return true))

(fn HealthChangeEEF
  (params (NewHealth :type ENUM_HealthStage%20Enum :default "NewEnumerator0") (Performer :type Actor%20Object%20Reference))
  (if (== Performer self)
    _
    (elif (Variables|EffectFlag|GetHealthChangeFlag)
      (return false)
      (else
        (Variables|EffectFlag|SetHealthChangeFlag true))))
  (return true))

(fn SellEEF
  (params (Performer :type Actor%20Object%20Reference))
  (Utilities|IsValid Performer
    (:Is%20Valid
      (if (== Performer self)
        _
        (else
          (if (Variables|EffectFlag|GetSellFlag) :!label _label
            (return false)
            (else
              (Variables|EffectFlag|SetSellFlag true))))))
    (:Is%20Not%20Valid
      (goto _label)))
  (return true))

(fn PlantPlacement
  (params (PlantsInRange :type Array%20of%20BP%20Plant%20Base%20Object%20References))
  (Placement|PickUpPlant)
  (bind _output_get (Variables|Default|SetPlantsInRange PlantsInRange))
  (for _array_element _output_get
    (Development|PrintString (Utilities|GetDisplayName _array_element))))

(fn PickUpPlant
  (bind _plantsinrange (Variables|Default|GetPlantsInRange))
  (Development|PrintString "unbind events here in pick up plant" true true "(R=1.000000,G=0.000000,B=0.037265,A=1.000000)")
  (Utilities|Array|Clear _plantsinrange)
  (Utilities|Array|Resize _plantsinrange 0))

(fn ChoosePlantstoPollinate
  (Development|PrintString "chose plants base")
  (bind _outactors (Actor|GetAllActorsOfClass "BP_Plant_Base_C"))
  (for _array_element _outactors
    (if (Utilities|Enum|Equal(Enum) (Variables|BP_Plant_Base_C|GetGrowthStage _array_element) "NewEnumerator3")
      (if (!= _array_element self)
        (Utilities|Array|AddUnique (LocalVariables|GetPlantsWithPollinateState) _array_element))))
  (return (LocalVariables|GetPlantsWithPollinateState)))

(fn SpecialAbility)

(fn SellF
  (params (HowMany :type Integer))
  (bind _ammount (Variables|Default|GetAmmount))
  (bind _aspsbp_mobile_player_state (Utilities|Casting|CastToPSBP_Mobile_PlayerState (Game|GetPlayerState 0)))
  (Default|PlantSell _aspsbp_mobile_player_state self HowMany)
  (Utilities|Struct|SetmembersinSTRUCT_PlantAmmount _ammount (- (.Ammount (Utilities|Struct|BreakSTRUCT_PlantAmmount _ammount)) 1))
  (Default|CallOnSell self)
  (if (<= (.Ammount (Utilities|Struct|BreakSTRUCT_PlantAmmount (Variables|Default|GetAmmount))) 0)
    (Actor|DestroyActor)))

(fn LimitArraytoCrossPollination
  (params (InputArray :type Array%20of%20BP%20Plant%20Base%20Object%20References))
  (for _array_element InputArray
    (if (== (Utilities|GetClass self) (Utilities|GetClass _array_element))
      (Utilities|Array|Add (LocalVariables|GetTempPlants) _array_element)
      (else
        (bind (_found_ _struct_plant) (CallFunction|GDFFind(byClass)PlantinDataTable (Utilities|GetClass _array_element)))
        (if _found_
          (if (.ReturnValue (Utilities|Map|Find (.CrossPollinationwithproduce (Utilities|Struct|BreakSTRUCT_PlantInfo _struct_plant)) (Utilities|GetClass _array_element)))
            (Utilities|Array|Add (LocalVariables|GetTempPlants) _array_element))))))
  (return (LocalVariables|GetTempPlants)))

(fn GetInfotoDisplay
  (bind _ammount (Variables|Default|GetAmmount))
  (return (.value (Variables|Default|GetValue)) (.ammount _ammount) (.maxammount _ammount) (Utilities|String|EnumtoString (Variables|Default|GetGrowthStage)) (Utilities|String|EnumtoString (Variables|Default|GetHealth)) (Variables|Default|GetTempHealthBuff) (Variables|Default|GetPlantsInRange)))