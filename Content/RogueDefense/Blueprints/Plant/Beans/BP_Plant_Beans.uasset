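; Beans plant in a roguelike-style defense game whose successful effects spread to every plant in the level, itself included.
; It overrides two effect functions, each calling the parent first and looping over all BP_Plant_Base actors if that succeeds.
; Health changes re-fire each plant's growth stage change at its current stage, while pollination adds a flat value to each.
; Neither override's return node is connected, so the parent's result is never passed back.
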(event EventBeginPlay
  (|CallParentFunction) ; This node is disabled and will not be called.\nDrag off pins to build functionality.
)

(event Collision|EventActorBeginOverlap
  (params (OtherActor :type Actor%20Object%20Reference)))

(event EventTick
  (params (DeltaSeconds :type Float%20%28single-precision%29)))

(fn ConstructionScript
  (|CallParentFunction))

(fn HealthChangeEEF
  (params (NewHealth :type ENUM_HealthStage%20Enum :default "NewEnumerator0") (Performer :type Actor%20Object%20Reference))
  (bind _canchildperform (|CallParentFunction NewHealth Performer))
  (if _canchildperform
    (bind _outactors (Actor|GetAllActorsOfClass "/Game/RogueDefense/Blueprints/Plant/Base/BP_Plant_Base.BP_Plant_Base_C"))
    (for _array_element _outactors
      (Default|CallOnGrowthStageChange _array_element (Variables|/Game/RogueDefense/Blueprints/Plant/Base/BP_Plant_Base.BP_Plant_Base_C|GetGrowthStage _array_element) self))))

(fn PollinateEEF
  (params (Performer :type Actor%20Object%20Reference))
  (bind _canchildperform (|CallParentFunction Performer))
  (if _canchildperform
    (bind _outactors (Actor|GetAllActorsOfClass "/Game/RogueDefense/Blueprints/Plant/Base/BP_Plant_Base.BP_Plant_Base_C"))
    (for _array_element _outactors
      (Default|AddValueF _array_element 5.0))))