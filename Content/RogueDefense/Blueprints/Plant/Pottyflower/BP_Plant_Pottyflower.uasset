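; Pottyflower plant for RogueDefense, extending the base plant's growth, sell and death effect functions, each gated on the parent's result.
; On growth with a pot applied, it passes the pot's value and amount bonuses to every plant in range.
; Selling adds one to its own amount.
; On death it spawns a random pot class on the closest pot grid lock, marking that lock occupied and caching it on the new pot.
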(event EventBeginPlay
  (|CallParentFunction) ; This node is disabled and will not be called.\nDrag off pins to build functionality.
)

(event Collision|EventActorBeginOverlap
  (params (OtherActor :type Actor%20Object%20Reference)))

(event EventTick
  (params (DeltaSeconds :type Float%20%28single-precision%29)))

(fn ConstructionScript
  (|CallParentFunction))

(fn GrowthEEF
  (params (NewGrowthStage :type ENUM_PlantGrowthStage%20Enum :default "NewEnumerator0") (Performer :type Actor%20Object%20Reference))
  (bind _canchildperform (|CallParentFunction NewGrowthStage Performer))
  (if _canchildperform
    (if (Variables|Default|GetPotApplied)
      (for _array_element (Variables|Default|GetPlantsInRange)
        (Default|AddValueF _array_element (Variables|Default|GetPotAddValue))
        (Default|AddAmountF _array_element (Variables|Default|GetPot%20Amount%20to%20Add) (Variables|Default|GetPot%20Max%20Amount%20to%20Add))))))

(fn SellEEF
  (params (Performer :type Actor%20Object%20Reference))
  (bind _canchildperform (|CallParentFunction Performer))
  (if _canchildperform
    (CallFunction|AddAmountF 1)))

(fn DeathEEF
  (params (Performer :type Actor%20Object%20Reference))
  (bind _canchildperform (|CallParentFunction Performer))
  (if _canchildperform
    (bind _gridlocation (CallFunction|FindClosestGridLock (Transformation|GetWorldLocation (Variables|Default|GetCube)) "Pot"))
    (Default|SetOccupied _gridlocation true)
    (bind _returnvalue (Game|SpawnActorfromClass (.OutItem (Utilities|Array|Random (Variables|Default|GetPotClasses))) (Transformation|GetActorTransform _gridlocation) "Undefined" "MultiplyWithRoot" 0 0))
    (Variables|/Game/RogueDefense/Blueprints/BP_TouchTest.BP_TouchTest_C|SetCachedGrid _returnvalue _gridlocation)))