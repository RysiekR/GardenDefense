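; Potato plant Blueprint for RogueDefense that buffs plants in range when it dies, is sold or grows.
; It overrides the parent's death, sell and growth effect functions, looping over PlantsInRange only when the parent call returns true.
; Death adds value to each plant equal to that plant's amount, selling raises amount, and growth raises max amount.
; The return nodes passing on the parent result never run.
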(event EventBeginPlay
  (|CallParentFunction) ; This node is disabled and will not be called.\nDrag off pins to build functionality.
)

(event Collision|EventActorBeginOverlap
  (params (OtherActor :type Actor%20Object%20Reference)))

(event EventTick
  (params (DeltaSeconds :type Float%20%28single-precision%29)))

(fn ConstructionScript
  (|CallParentFunction))

(fn DeathEEF
  (params (Performer :type Actor%20Object%20Reference))
  (bind _canchildperform (|CallParentFunction Performer))
  (if _canchildperform
    (for _array_element (Variables|Default|GetPlantsInRange)
      (Default|AddValueF _array_element (Math|Conversions|ToFloat(Integer) (.Ammount (Utilities|Struct|BreakSTRUCT_PlantAmmount (Variables|/Game/RogueDefense/Blueprints/Plant/Base/BP_Plant_Base.BP_Plant_Base_C|GetAmmount _array_element))))))))

(fn SellEEF
  (params (Performer :type Actor%20Object%20Reference))
  (bind _canchildperform (|CallParentFunction Performer))
  (if _canchildperform
    (for _array_element (Variables|Default|GetPlantsInRange)
      (Default|AddAmountF _array_element 1))))

(fn GrowthEEF
  (params (NewGrowthStage :type ENUM_PlantGrowthStage%20Enum :default "NewEnumerator0") (Performer :type Actor%20Object%20Reference))
  (bind _canchildperform (|CallParentFunction NewGrowthStage Performer))
  (if _canchildperform
    (for _array_element (Variables|Default|GetPlantsInRange)
      (Default|AddAmountF _array_element 0 1))))