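; Money Tree plant for RogueDefense that overrides the growth, sell and death effect functions, each gated on its parent's result.
; Growth adds the other plants' summed value divided by the total plant count, itself included.
; Selling calls OnSell with itself once per other plant.
; Death copies its value onto the highest-value plant found, despite the CheapestPlant variable name, without excluding itself.
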(event EventBeginPlay
  (|CallParentFunction) ; This node is disabled and will not be called.\nDrag off pins to build functionality.
)

(event Collision|EventActorBeginOverlap
  (params (OtherActor :type Actor%20Object%20Reference)))

(event EventTick
  (params (DeltaSeconds :type Float%20%28single-precision%29)))

(fn ConstructionScript
  (|CallParentFunction))

(fn GrowthEEF
  (params (NewGrowthStage :type ENUM_PlantGrowthStage%20Enum :default "NewEnumerator0") (Performer :type Actor%20Object%20Reference))
  (bind _canchildperform (|CallParentFunction NewGrowthStage Performer))
  (if _canchildperform
    (Variables|Default|SetSumValueOfAllPlants 0.0)
    (bind _outactors (Actor|GetAllActorsOfClass "/Game/RogueDefense/Blueprints/Plant/Base/BP_Plant_Base.BP_Plant_Base_C"))
    (for _array_element _outactors
      (if (not (== _array_element self))
        (Variables|Default|SetSumValueOfAllPlants (+ (Variables|Default|GetSumValueOfAllPlants) (.value (Variables|/Game/RogueDefense/Blueprints/Plant/Base/BP_Plant_Base.BP_Plant_Base_C|GetValue _array_element))))))
    (CallFunction|AddValueF (Math|Float|SafeDivide (Variables|Default|GetSumValueOfAllPlants) (Math|Conversions|ToFloat(Integer) (Utilities|Array|Length _outactors))))))

(fn SellEEF
  (params (Performer :type Actor%20Object%20Reference))
  (bind _canchildperform (|CallParentFunction Performer))
  (if _canchildperform
    (bind _outactors (Actor|GetAllActorsOfClass "/Game/RogueDefense/Blueprints/Plant/Base/BP_Plant_Base.BP_Plant_Base_C"))
    (for _array_element _outactors
      (if (not (== _array_element self))
        (Default|CallOnSell self)))))

(fn DeathEEF
  (params (Performer :type Actor%20Object%20Reference))
  (bind _canchildperform (|CallParentFunction Performer))
  (if _canchildperform
    (bind _outactors (Actor|GetAllActorsOfClass "/Game/RogueDefense/Blueprints/Plant/Base/BP_Plant_Base.BP_Plant_Base_C"))
    (if (Utilities|Array|IsNotEmpty _outactors)
      (Variables|Default|SetCheapestPlant 0)
      (for _array_element _outactors
        (bind _cheapestplant (Variables|Default|GetCheapestPlant)
          (:then
            (if (< (.Value (Utilities|Struct|BreakSTRUCT_PlantValue (Variables|/Game/RogueDefense/Blueprints/Plant/Base/BP_Plant_Base.BP_Plant_Base_C|GetValue _cheapestplant))) (.Value (Utilities|Struct|BreakSTRUCT_PlantValue (Variables|/Game/RogueDefense/Blueprints/Plant/Base/BP_Plant_Base.BP_Plant_Base_C|GetValue _array_element))))
              (Variables|Default|SetCheapestPlant _array_element)))
          (:else
            (Variables|Default|SetCheapestPlant _array_element))))
      (bind _cheapestplant_2 (Variables|Default|GetCheapestPlant)
        (:then
          (Utilities|Struct|SetmembersinSTRUCT_PlantValue (Variables|/Game/RogueDefense/Blueprints/Plant/Base/BP_Plant_Base.BP_Plant_Base_C|GetValue _cheapestplant_2) (.value (Variables|Default|GetValue))))
        (:else)))))