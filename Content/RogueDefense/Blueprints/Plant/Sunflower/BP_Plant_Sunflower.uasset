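; Sunflower plant for Rogue Defense that gives chance-based buffs to itself and nearby plants through overridden effect hooks.
; Each hook calls its parent version first and applies its effect only if that succeeds.
; On death or sale, it rolls separately for each plant in range, granting temporary HP or raising an amount and its maximum respectively.
; On growth, it may give itself temporary HP.
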(event EventBeginPlay
  (|CallParentFunction) ; This node is disabled and will not be called.\nDrag off pins to build functionality.
)

(event Collision|EventActorBeginOverlap
  (params (OtherActor :type Actor%20Object%20Reference)))

(event EventTick
  (params (DeltaSeconds :type Float%20%28single-precision%29)))

(fn ConstructionScript
  (|CallParentFunction))

(fn DeathEEF
  (params (Performer :type Actor%20Object%20Reference))
  (bind _canchildperform (|CallParentFunction Performer))
  (if _canchildperform
    (for _array_element (Variables|Default|GetPlantsInRange)
      (if (<= (Math|Random|RandomIntegerinRange 0 99) 33)
        (Default|AddTempHP _array_element "NewEnumerator1" (.Value (Utilities|Map|Find (Variables|Default|GetTempHealthBuff) "NewEnumerator1")))))))

(fn SellEEF
  (params (Performer :type Actor%20Object%20Reference))
  (bind _canchildperform (|CallParentFunction Performer))
  (if _canchildperform
    (for _array_element (Variables|Default|GetPlantsInRange)
      (if (<= (Math|Random|RandomIntegerinRange 0 99) 25)
        (Default|AddAmountF _array_element 1 1)))))

(fn GrowthEEF
  (params (NewGrowthStage :type ENUM_PlantGrowthStage%20Enum :default "NewEnumerator0") (Performer :type Actor%20Object%20Reference))
  (bind _canchildperform (|CallParentFunction NewGrowthStage Performer))
  (if _canchildperform
    (if (<= (Math|Random|RandomIntegerinRange 0 99) 50)
      (CallFunction|AddTempHP "NewEnumerator1" 1))))