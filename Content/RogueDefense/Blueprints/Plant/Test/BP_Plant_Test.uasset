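; Test plant Blueprint for RogueDefense that exercises the parent plant's overridable death, pollination, growth and placement functions, mostly passing through with debug prints.
; It overrides pollination target choice to gather unique in-range plants at one specific growth stage.
; On placement it binds to each nearby plant's growth-stage dispatcher, apparently for SpecialAbilityTest, a stub ability that only prints when another plant grows.
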(event EventBeginPlay
  (|CallParentFunction))

(event Collision|EventActorBeginOverlap
  (params (OtherActor :type Actor%20Object%20Reference)))

(event EventTick
  (params (DeltaSeconds :type Float%20%28single-precision%29)))

(fn ConstructionScript
  (|CallParentFunction))

(fn DeathEEF
  (params (Performer :type Actor%20Object%20Reference))
  (bind _canchildperform (|CallParentFunction Performer))
  (if _canchildperform
    (Development|PrintString "child goodbye")))

(fn PollinateEEF
  (params (Performer :type Actor%20Object%20Reference))
  (bind _canchildperform (|CallParentFunction Performer))
  (if _canchildperform
    _))

(fn GrowthEEF
  (params (NewGrowthStage :type ENUM_PlantGrowthStage%20Enum :default "NewEnumerator0") (Performer :type Actor%20Object%20Reference))
  (bind _canchildperform (|CallParentFunction NewGrowthStage Performer))
  (if _canchildperform
    (return _canchildperform)))

(fn ChoosePlantstoPollinate
  (bind _temppolinatableplants (LocalVariables|GetTempPolinatablePlants))
  (Utilities|Array|Clear (LocalVariables|GetTempPolinatablePlants))
  (for _array_element (Variables|Default|GetPlantsInRange)
    (if (Utilities|Enum|Equal(Enum) (Variables|/Game/RogueDefense/Blueprints/Plant/Base/BP_Plant_Base.BP_Plant_Base_C|GetGrowthStage _array_element) "NewEnumerator3")
      (Utilities|Array|AddUnique (LocalVariables|GetTempPolinatablePlants) _array_element)))
  (Development|PrintText (Utilities|Text|FormatText "test,chooseplants to pollinate, length:{a}" (Utilities|Array|Length _temppolinatableplants)))
  (return _temppolinatableplants))

(fn PollinateF
  (params (ChooseFrom :type Array%20of%20BP%20Plant%20Base%20Object%20References))
  (|CallParentFunction ChooseFrom))

(fn PlantPlacement
  (params (PlantsInRange :type Array%20of%20BP%20Plant%20Base%20Object%20References))
  (|CallParentFunction PlantsInRange)
  (for _array_element PlantsInRange
    (EventDispatchers|BindEventtoOnGrowthStageChange _array_element (EventDispatchers|CreateEvent :!event SpecialAbilityTest)))
  (return))

(fn SpecialAbilityTest
  (params (NewGrowthStage :type ENUM_PlantGrowthStage%20Enum :default "NewEnumerator0") (Performer :type Actor%20Object%20Reference))
  (Development|PrintString "executed special ability on growth dispatcher from other"))