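; BP_Plant_Rose is the Rose plant in RogueDefense, a child Blueprint whose effects act on the plants in its range.
; It overrides the parent's growth, health-change and sell effect functions, acting only when the parent call returns true.
; Growth grants temporary HP to itself and its neighbours, health change calls each neighbour's CallOnDeath with the Rose as argument, and selling adds value to each neighbour.
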(event EventBeginPlay
  (|CallParentFunction) ; This node is disabled and will not be called.\nDrag off pins to build functionality.
)

(event Collision|EventActorBeginOverlap
  (params (OtherActor :type Actor%20Object%20Reference)))

(event EventTick
  (params (DeltaSeconds :type Float%20%28single-precision%29)))

(fn ConstructionScript
  (|CallParentFunction))

(fn GrowthEEF
  (params (NewGrowthStage :type ENUM_PlantGrowthStage%20Enum :default "NewEnumerator0") (Performer :type Actor%20Object%20Reference))
  (bind _canchildperform (|CallParentFunction NewGrowthStage Performer))
  (if _canchildperform
    (for _array_element (Variables|Default|GetPlantsInRange)
      (Default|AddTempHP _array_element "NewEnumerator0" 1))
    (CallFunction|AddTempHP "NewEnumerator0" 1)))

(fn HealthChangeEEF
  (params (NewHealth :type ENUM_HealthStage%20Enum :default "NewEnumerator0") (Performer :type Actor%20Object%20Reference))
  (bind _canchildperform (|CallParentFunction NewHealth Performer))
  (if _canchildperform
    (for _array_element (Variables|Default|GetPlantsInRange)
      (Default|CallOnDeath _array_element self))))

(fn SellEEF
  (params (Performer :type Actor%20Object%20Reference))
  (bind _canchildperform (|CallParentFunction Performer))
  (if _canchildperform
    (for _array_element (Variables|Default|GetPlantsInRange)
      (Default|AddValueF _array_element 5.0))))