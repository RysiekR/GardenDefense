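; Tomato plant for RogueDefense that overrides the parent plant's death, growth and sell effects, each acting only when the parent call returns true.
; Growth adds the plant's base value to itself, and death adds its current value to a random plant in range.
; Selling calls OnSell on every plant in range, passing itself.
; The return nodes in all three overrides are unreachable, so the parent result is not passed back.
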(event EventBeginPlay
  (|CallParentFunction) ; This node is disabled and will not be called.\nDrag off pins to build functionality.
)

(event Collision|EventActorBeginOverlap
  (params (OtherActor :type Actor%20Object%20Reference)))

(event EventTick
  (params (DeltaSeconds :type Float%20%28single-precision%29)))

(fn ConstructionScript
  (|CallParentFunction))

(fn DeathEEF
  (params (Performer :type Actor%20Object%20Reference))
  (bind _canchildperform (|CallParentFunction Performer))
  (if _canchildperform
    (Default|AddValueF (.OutItem (Utilities|Array|Random (Variables|Default|GetPlantsInRange))) (.Value (Utilities|Struct|BreakSTRUCT_PlantValue (Variables|Default|GetValue))))))

(fn GrowthEEF
  (params (NewGrowthStage :type ENUM_PlantGrowthStage%20Enum :default "NewEnumerator0") (Performer :type Actor%20Object%20Reference))
  (bind _canchildperform (|CallParentFunction NewGrowthStage Performer))
  (if _canchildperform
    (CallFunction|AddValueF (.BaseValue (Utilities|Struct|BreakSTRUCT_PlantValue (Variables|Default|GetValue))))))

(fn SellEEF
  (params (Performer :type Actor%20Object%20Reference))
  (bind _canchildperform (|CallParentFunction Performer))
  (if _canchildperform
    (for _array_element (Variables|Default|GetPlantsInRange)
      (Default|CallOnSell _array_element self))))