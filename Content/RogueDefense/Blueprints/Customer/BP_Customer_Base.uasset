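; Base customer character that picks a random plant in the level, walks to it, buys it and then disappears.
; On BeginPlay it chooses among all BP_Plant_Base actors and sends its AI controller toward the choice with MoveToActor.
; On Tick, while movement is idle, a sphere trace checks for that plant nearby, then calls its SellF and destroys the customer.
; Retargeting logic with a Niagara effect exists but is disconnected.
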(event EventBeginPlay
  (CallFunction|ChoosePlanttoBuy)
  (CallFunction|GoTowordsPlant))

(event EventTick
  (params (DeltaSeconds :type Float%20%28single-precision%29))
  (bind _capsulecomponent (Variables|Collision|GetCapsuleComponent))
  (bind _returnvalue (Transformation|GetWorldLocation _capsulecomponent))
  (if (> (Actor|GetGameTimeSinceCreation self) 0.1)
    (switch Utilities|FlowControl|Switch|SwitchonEPathFollowingStatus (Class|AIController|GetMoveStatus (AI|GetAIController self))
      (:Idle
        (bind _outhits (Collision|MultiSphereTraceByChannel _returnvalue _returnvalue 2e+02 "TraceTypeQuery1" false 0 "ForDuration"))
        (bind (_array_element _array_index) (Utilities|Array|ForEachLoopwithBreak _outhits :!label _label)
          (:LoopBody
            (if (== (.HitActor (Collision|BreakHitResult _array_element)) (Variables|Default|GetChosenPlant))
              (Development|PrintString "at plant location")
              (bind _asbp_plant_base (Utilities|Casting|CastToBP_Plant_Base (.HitActor (Collision|BreakHitResult _array_element))))
              (CallFunction|BuyPlant _asbp_plant_base)
              (goto _label Break))))))))

(fn ConstructionScript)

(fn ChoosePlanttoBuy
  (bind _outactors (Actor|GetAllActorsOfClass "/Game/RogueDefense/Blueprints/Plant/Base/BP_Plant_Base.BP_Plant_Base_C"))
  (Variables|Default|SetChosenPlant (.OutItem (Utilities|Array|Random _outactors))))

(fn BuyPlant
  (params (Plant :type BP%20Plant%20Base%20Object%20Reference))
  (Default|SellF Plant 1)
  (CallFunction|Disappear))

(fn GoTowordsPlant
  (bind _asaicontroller (Utilities|Casting|CastToAIController (Pawn|GetController)))
  (bind _returnvalue (AI|Navigation|MovetoActor _asaicontroller (Variables|Default|GetChosenPlant) 1e+02 true true true 0))
  (switch Utilities|FlowControl|Switch|SwitchonEPathFollowingRequestResult _returnvalue
    (:Failed
      (Development|PrintString "Failed pathing"))
    (:AlreadyAtGoal
      (Development|PrintString "already at goal path"))
    (:RequestSuccessful
      (Development|PrintString "path found... going"))))

(fn Disappear
  (Development|PrintString "customer bought, now exits")
  (Actor|DestroyActor))