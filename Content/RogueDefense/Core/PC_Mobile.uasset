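; Player controller for RogueDefense's mobile mode that shows the cursor and relays touch input.
; Touch move and release fire the TouchMove and StopTouching dispatchers, with moves passing the touch location.
; A touch-begin binding prints the touched actor.
; Debug keys P, G and B cast to GM_Mobile to trigger Pollinate, Grow and PopulateBench.
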(event Custom|OnInputTouchBegin_Event
  (params (FingerIndex :type ETouchIndex%20Enum :default "Touch1") (TouchedActor :type Actor%20Object%20Reference))
  (Development|PrintText (Utilities|Text|FormatText "touching:{a}" TouchedActor)))

(event EventBeginPlay
  (Variables|Default|SetbShowMouseCursor true)
  (EventDispatchers|AssignOnInputTouchBegin (delegate Custom|OnInputTouchBegin_Event)))

(event Input|KeyboardEvents|DebugKeyP
  (params (Key :type Key%20Structure :default "None") (ActionValue :type Input%20Action%20Value%20Structure))
  (:Pressed
    (bind _asgm_mobile (Utilities|Casting|CastToGM_Mobile (Game|GetGameMode)))
    (Default|Pollinate _asgm_mobile)))

(event Input|KeyboardEvents|DebugKeyG
  (params (Key :type Key%20Structure :default "None") (ActionValue :type Input%20Action%20Value%20Structure))
  (:Pressed
    (bind _asgm_mobile (Utilities|Casting|CastToGM_Mobile (Game|GetGameMode)))
    (Default|Grow _asgm_mobile)))

(event Input|KeyboardEvents|DebugKeyB
  (params (Key :type Key%20Structure :default "None") (ActionValue :type Input%20Action%20Value%20Structure))
  (:Pressed
    (bind _asgm_mobile (Utilities|Casting|CastToGM_Mobile (Game|GetGameMode)))
    (Default|PopulateBench _asgm_mobile)))

(event Input|TouchEvents|InputTouch
  (params (Location :type Vector) (FingerIndex :type ETouchIndex%20Enum))
  (:Released
    (Default|CallStopTouching))
  (:Moved
    (Default|CallTouchMove Location)))

(fn ConstructionScript)