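; GM_Mobile, apparently the mobile game mode for RogueDefense, exposes events that drive plant growth, pollination and bench filling.
; Grow and Pollinate first have every BP_Plant_Base refresh its plants in range, then call the matching action on all plants.
; PopulateBench spawns a BP_Plant_Test on each free BP_Bench grid cell, marks it occupied and caches the cell on the plant.
; BeginPlay is empty; a looping timer is left unconnected.
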(event Custom|Grow
  (CallFunction|UpdatePlantsinRange)
  (bind _outactors (Actor|GetAllActorsOfClass "/Game/RogueDefense/Blueprints/Plant/Base/BP_Plant_Base.BP_Plant_Base_C"))
  (Default|Grow _outactors))

(event Custom|Pollinate
  (CallFunction|UpdatePlantsinRange)
  (bind _outactors (Actor|GetAllActorsOfClass "/Game/RogueDefense/Blueprints/Plant/Base/BP_Plant_Base.BP_Plant_Base_C"))
  (Default|Pollinate _outactors))

(event Custom|UpdatePlantsInRange
  (bind _outactors (Actor|GetAllActorsOfClass "/Game/RogueDefense/Blueprints/Plant/Base/BP_Plant_Base.BP_Plant_Base_C"))
  (for _array_element _outactors
    (Default|GetPlantsinRange _array_element)))

(event Custom|PopulateBench
  (bind _returnvalue (Actor|GetActorOfClass "/Game/RogueDefense/Blueprints/BP_Bench.BP_Bench_C"))
  (for _array_element (Variables|/Game/RogueDefense/Blueprints/BP_Bench.BP_Bench_C|GetBenchGrid _returnvalue)
    (if (not (Variables|/Game/RogueDefense/Blueprints/GridLockPosition/BP_GridLockPosition.BP_GridLockPosition_C|GetOccupied? _array_element))
      (bind _returnvalue_2 (Game|SpawnActorfromClass "/Game/RogueDefense/Blueprints/Plant/Test/BP_Plant_Test.BP_Plant_Test_C" (Transformation|GetActorTransform _array_element) "Undefined" "MultiplyWithRoot" 0 "Test" 0))
      (Default|SetOccupied _array_element true)
      (Variables|/Game/RogueDefense/Blueprints/BP_TouchTest.BP_TouchTest_C|SetCachedGrid _returnvalue_2 _array_element))))

(event EventBeginPlay)

(fn ConstructionScript)